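; Player controller that builds a grid of TileMap_Brick_BP actors on BeginPlay and randomly re-materials bricks on left click.
; Materials load from a data table, with one picked at random as the spawn default.
; Nested loops chain bricks from each predecessor's next-brick and next-line arrow components.
; Clicks use a cursor object-type trace; CleanTileMap destroys the TileMap array's actors, though spawned bricks are never added to it.
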(event EventBeginPlay
  (CallFunction|LoadTileMapsMaterials)
  (CallFunction|GenereteTileMap))

(event EventTick
  (params (DeltaSeconds :type Float%20%28single-precision%29)))

(event Input|MouseEvents|LeftMouseButton
  (params (Key :type Key%20Structure :default "AnyKey"))
  (bind _selectebleobjectsingame (Variables|Default|GetSelectebleObjectsInGame))
  (bind _hitresult (Class|PlayerController|GetHitResultUnderCursorforObjects _selectebleobjectsingame true))
  (:Pressed
    (Utilities|IsValid (.hitactor _hitresult)
      (:Is%20Valid
        (bind _astile_map_brick_bp (Utilities|Casting|CastToTileMap_Brick_BP (.hitactor _hitresult)))
        (CallFunction|ChangeTileMapElementMaterial _astile_map_brick_bp)))))

(fn ConstructionScript)

(fn GenereteTileMap
  (CallFunction|CleanTileMap)
  (for _index (range 1 (Variables|Default|GetTileMapWidth))
    (bind _newstartlinebrick (CallFunction|AddNewTileMapLine (LocalVariables|GetCurrentStartLineBrick)))
    (bind _output_get (LocalVariables|SetCurrentStartLineBrick _newstartlinebrick))
    (LocalVariables|SetCurrentBrick _output_get)
    (for _index_2 (range 1 (Variables|Default|GetTileMapHeidth))
      (bind _newelement (CallFunction|AddNewTileMapElement (LocalVariables|GetCurrentBrick)))
      (LocalVariables|SetCurrentBrick _newelement))))

(fn AddNewTileMapElement
  (params (PreviusElement :type Tile%20Map%20Brick%20BP%20Object%20Reference))
  (bind _returnvalue (Game|SpawnActorfromClass "/Game/Blueprints/TileMap_Brick_BP.TileMap_Brick_BP_C" (Math|Transform|MakeTransform (Transformation|GetWorldLocation (Variables|/Game/Blueprints/TileMap_Brick_BP.TileMap_Brick_BP_C|GetArrow_NextBrickPosition PreviusElement))) "AlwaysSpawn" 0 (.material (Variables|Default|GetDefaultMaterialStuct)) 0))
  (return _returnvalue))

(fn AddNewTileMapLine
  (params (PreviusStartLineBrick :type Tile%20Map%20Brick%20BP%20Object%20Reference))
  (Utilities|IsValid PreviusStartLineBrick
    (:Is%20Valid
      (LocalVariables|SetLocation (Transformation|GetWorldLocation (Variables|/Game/Blueprints/TileMap_Brick_BP.TileMap_Brick_BP_C|GetArrow_NextLinePosition PreviusStartLineBrick))))
    (:Is%20Not%20Valid
      _))
  (bind _returnvalue (Game|SpawnActorfromClass "/Game/Blueprints/TileMap_Brick_BP.TileMap_Brick_BP_C" (Math|Transform|MakeTransform (LocalVariables|GetLocation)) "AlwaysSpawn" 0 (.material (Variables|Default|GetDefaultMaterialStuct)) 0))
  (return _returnvalue))

(fn CleanTileMap
  (for _array_element (Variables|Default|GetTileMap)
    (Actor|DestroyActor _array_element))
  (Utilities|Array|Clear (Variables|Default|GetTileMap)))

(fn LoadTileMapsMaterials
  (bind _tilemapmaterials (Variables|Default|GetTileMapMaterials))
  (bind _returnvalue (Utilities|Array|Length _tilemapmaterials))
  (Utilities|Array|Clear (Variables|Default|GetTileMapMaterials))
  (bind _outrownames (DataTable|GetDataTableRowNames "/Game/Data/TieMapMaterials.TieMapMaterials"))
  (for _array_element _outrownames
    (bind _returnvalue_2 (Utilities|GetDataTableRow "/Game/Data/TieMapMaterials.TieMapMaterials" _array_element)
      (:then
        (Utilities|Array|Add (Variables|Default|GetTileMapMaterials) _returnvalue_2))))
  (if (> _returnvalue 0)
    (Variables|Default|SetDefaultMaterialStuct (Utilities|Array|Get(acopy) (Variables|Default|GetTileMapMaterials) (Math|Random|RandomIntegerinRange 0 (- _returnvalue 1))))))

(fn ChangeTileMapElementMaterial
  (params (Element :type Tile%20Map%20Brick%20BP%20Object%20Reference))
  (bind _tilemapmaterials (Variables|Default|GetTileMapMaterials))
  (bind _returnvalue (Utilities|Array|Length _tilemapmaterials))
  (Utilities|IsValid Element
    (:Is%20Valid
      (if (> _returnvalue 0)
        (Default|UpdateMaterial Element (.material (Utilities|Array|Get(acopy) (Variables|Default|GetTileMapMaterials) (Math|Random|RandomIntegerinRange 0 (- _returnvalue 1)))))))))